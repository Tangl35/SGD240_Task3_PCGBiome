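; BP_ClimateManager is an unfinished climate manager Actor holding a CurrentClimate struct of temperature, wind, moisture and precipitation.
; Tick only assigns CurrentClimate back to itself, so the climate never changes.
; A disconnected node chain drafts a time-based sine for temperature, random wind and moisture drift, and moisture-dependent precipitation with zeroed random ranges.
; The construction script and NewFunction are empty.
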(event `self.ReceiveTick`
  (params (DeltaSeconds :type "Float (single-precision)"))
  ; Update Climate Function
  (bind _output_get (set `self.CurrentClimate` (`self.CurrentClimate`))))

(fn `NewFunction`)

(fn `UserConstructionScript`)