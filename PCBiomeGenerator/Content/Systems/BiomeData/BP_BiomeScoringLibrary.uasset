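; Biome scoring function library that rates forest, grassland, freshwater, cliff, road/fence and fog zone from terrain and climate inputs for PCG points.
; Each Score function returns a clamped weighted sum, which BlendBiomeScores writes onto points as float attributes.
; ChooseFinalBiome is unfinished: it reads "BiomeScore_" names though Blend writes "BomeScore_", and sets FinalBiome without a computed value.
; Weight normalization and priority-override selection logic exist but are disconnected.
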(fn ScoreForest
  (params (Temperature :type Float%20%28double-precision%29) (Humidity :type Float%20%28double-precision%29) (Slope :type Float%20%28double-precision%29) (WaterProximity :type Float%20%28double-precision%29))
  (return (Math|Float|Clamp(Float) (+ (+ (+ (* (Math|Float|Max(Float) (- Temperature 0.35) 0.0) 1.5) (* (Math|Float|Max(Float) (- Humidity 0.55) 0.0) 2.0)) (* (Math|Float|Clamp(Float) (- 1.0 Slope)) 0.6)) (* WaterProximity 0.3)))))

(fn ScoreGrassland
  (params (Temperature :type Float%20%28double-precision%29) (Humidity :type Float%20%28double-precision%29) (Slope :type Float%20%28double-precision%29) (WaterProximity :type Float%20%28double-precision%29))
  (return (Math|Float|Clamp(Float) (+ (+ (+ (* (Math|Float|Max(Float) (- Temperature 0.25) 0.0) 1.0) (* (Math|Float|Max(Float) (- 0.6 Humidity) 0.0) 0.8)) (* (- 1.0 Slope) 4.0)) (* WaterProximity 0.5)))))

(fn ScoreFreshwater
  (params (Temperature :type Float%20%28double-precision%29) (Humidity :type Float%20%28double-precision%29) (Slope :type Float%20%28double-precision%29) (WaterProximity :type Float%20%28double-precision%29))
  (return (Math|Float|Clamp(Float) (+ (* (- Slope 0.0) 0.3) (* WaterProximity 2.0)))))

(fn ScoreCliff
  (params (Slope :type Float%20%28double-precision%29) (Elevation :type Float%20%28double-precision%29))
  (return (Math|Float|Clamp(Float) (+ (* (- Slope 0.6) 2.0) (* Elevation 0.1)))))

(fn ScoreRoadFence
  (params (Temperature :type Float%20%28double-precision%29) (Humidity :type Float%20%28double-precision%29) (Slope :type Float%20%28double-precision%29))
  (return (Math|Float|Clamp(Float) (* Slope 0.4))))

(fn ScoreFogZone
  (params (Humidity :type Float%20%28double-precision%29) (Elevation :type Float%20%28double-precision%29) (TimeOfDay :type Float%20%28double-precision%29))
  (return (Math|Float|Clamp(Float) (+ (+ (* Humidity 0.8) (* (- 1.0 Elevation) 0.1)) (* TimeOfDay 0.1)))))

(fn BlendBiomeScores
  (params (ScoreForest :type Float%20%28double-precision%29) (ScoreGrassland :type Float%20%28double-precision%29) (ScoreFreshwater :type Float%20%28double-precision%29) (ScoreCliff :type Float%20%28double-precision%29) (ScoreRoadFence :type Float%20%28double-precision%29) (ScoreFogZone :type Float%20%28double-precision%29) (PCGPoints :type Array%20of%20PCG%20Point%20Structures))
  (for _array_element PCGPoints
    (PCG|Metadata|SetFloatAttribute _array_element 0 "BomeScore_Road" ScoreRoadFence)
    (PCG|Metadata|SetFloatAttribute _array_element 0 "BomeScore_Cliff" ScoreCliff)
    (PCG|Metadata|SetFloatAttribute _array_element 0 "BomeScore_Freshwater" ScoreFreshwater)
    (PCG|Metadata|SetFloatAttribute _array_element 0 "BomeScore_Forest" ScoreForest)
    (PCG|Metadata|SetFloatAttribute _array_element 0 "BomeScore_Grassland" ScoreGrassland)
    (PCG|Metadata|SetFloatAttribute _array_element 0 "BomeScore_FogZone" ScoreFogZone)))

(fn ChooseFinalBiome
  (params (WForest :type Float%20%28double-precision%29) (WGrassland :type Float%20%28double-precision%29) (WFreshwater :type Float%20%28double-precision%29) (WCliff :type Float%20%28double-precision%29) (WRoadFence :type Float%20%28double-precision%29) (WFogDensity :type Float%20%28double-precision%29) (Points :type Array%20of%20PCG%20Point%20Structures))
  ;[0.15 0.15 0.15 0.5] Each point to store a final EBiomeType attribute
  (for _array_element Points :!label _label
    (bind _returnvalue (PCG|Metadata|GetFloatAttributebyMetadataKey (.MetadataEntry (Utilities|Struct|BreakPCGPoint _array_element)) 0 "BiomeScore_Road"))
    (bind _returnvalue_2 (PCG|Metadata|GetFloatAttributebyMetadataKey (.MetadataEntry (Utilities|Struct|BreakPCGPoint _array_element)) 0 "BiomeScore_Cliff"))
    (bind _returnvalue_3 (PCG|Metadata|GetFloatAttributebyMetadataKey (.MetadataEntry (Utilities|Struct|BreakPCGPoint _array_element)) 0 "BiomeScore_Freshwater"))
    (bind _returnvalue_4 (PCG|Metadata|GetFloatAttributebyMetadataKey (.MetadataEntry (Utilities|Struct|BreakPCGPoint _array_element)) 0 "BiomeScore_Forest"))
    (bind _returnvalue_5 (PCG|Metadata|GetFloatAttributebyMetadataKey (.MetadataEntry (Utilities|Struct|BreakPCGPoint _array_element)) 0 "BiomeScore_Grassland"))
    (bind _returnvalue_6 (PCG|Metadata|GetFloatAttributebyMetadataKey (.MetadataEntry (Utilities|Struct|BreakPCGPoint _array_element)) 0 "BiomeScore_FogZone"))
    (PCG|Metadata|SetInteger32AttributebyMetadataKey (.MetadataEntry (Utilities|Struct|BreakPCGPoint _array_element)) 0 "FinalBiome" 0)
    (goto _label))
  (Utilities|Array|Add 0 (Utilities|Struct|MakePCGPoint (.Transform (Utilities|Struct|BreakPCGPoint _array_element)) (.Density (Utilities|Struct|BreakPCGPoint _array_element)) (.BoundsMin (Utilities|Struct|BreakPCGPoint _array_element)) (.BoundsMax (Utilities|Struct|BreakPCGPoint _array_element)) (.Color (Utilities|Struct|BreakPCGPoint _array_element)) (.Steepness (Utilities|Struct|BreakPCGPoint _array_element)) (.Seed (Utilities|Struct|BreakPCGPoint _array_element)))))