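; A custom PCG element meant to tag points with climate data for biome generation, marked as unworkable in favor of a ClimateIntegration PCG graph.
; It loops over input points, querying the climate manager at each location to set temperature, humidity, fog density, slope, elevation and water proximity attributes.
; Each attribute makes its own climate query, and the rebuilt points are collected but never written to an output.
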(fn ExecutewithContext
  (params (InContext :type PCG%20Context%20Structure%20%28by%20ref%29) (Input :type PCG%20Data%20Collection%20Structure%20%28by%20ref%29))
  ;[0.15 0.15 0.15 0.5] Convert input data to an array
  (bind _returnvalue (Class|PCGBlueprintHelpers|GetInputData InContext)) ; In
  (bind _aspcgpoint_data (Utilities|Casting|CastToPCGPointData _returnvalue))
  (bind _output_get (Variables|Default|SetOutputPoints (Utilities|Array|MakeArray (stale _array_element))))
  (for _array_element (SpatialData|GetPoints _aspcgpoint_data) :!label _label ; For each input convert to metadata attribute
    ;[0.15 0.15 0.15 0.5] Convert points to Metadata Attributes
    (PCG|Metadata|SetFloatAttribute _array_element 0 "Temperature" (.temperature (Default|GetClimateatWorldPosition (Variables|Default|GetBP_ClimateManager) (.location (.Transform (Utilities|Struct|BreakPCGPoint _array_element))) 1.0)))
    (PCG|Metadata|SetFloatAttribute _array_element 0 "Humidity" (.humidity (Default|GetClimateatWorldPosition (Variables|Default|GetBP_ClimateManager) (.location (.Transform (Utilities|Struct|BreakPCGPoint _array_element))) 1.0)))
    (PCG|Metadata|SetFloatAttribute _array_element 0 "FogDensity" (.fogdensity (Default|GetClimateatWorldPosition (Variables|Default|GetBP_ClimateManager) (.location (.Transform (Utilities|Struct|BreakPCGPoint _array_element))) 1.0)))
    (PCG|Metadata|SetFloatAttribute _array_element 0 "SlopeFactor" (.slopefactor (Default|GetClimateatWorldPosition (Variables|Default|GetBP_ClimateManager) (.location (.Transform (Utilities|Struct|BreakPCGPoint _array_element))) 1.0)))
    (PCG|Metadata|SetFloatAttribute _array_element 0 "Elevation" (.elevation (Default|GetClimateatWorldPosition (Variables|Default|GetBP_ClimateManager) (.location (.Transform (Utilities|Struct|BreakPCGPoint _array_element))) 1.0)))
    (PCG|Metadata|SetFloatAttribute _array_element 0 "WaterProximity" (.waterproximity (Default|GetClimateatWorldPosition (Variables|Default|GetBP_ClimateManager) (.location (.Transform (Utilities|Struct|BreakPCGPoint _array_element))) 1.0)))
    (Utilities|Array|Add _output_get (Utilities|Struct|MakePCGPoint (.Transform (Utilities|Struct|BreakPCGPoint _array_element)) (.Density (Utilities|Struct|BreakPCGPoint _array_element)) (.BoundsMin (Utilities|Struct|BreakPCGPoint _array_element)) (.BoundsMax (Utilities|Struct|BreakPCGPoint _array_element)) "(X=1.000000,Y=1.000000,Z=1.000000,W=1.000000)" 0.5 0))
    (goto _label))
  ;[0.15 0.15 0.15 0.5] Cannot work - moving to PCGGraph CLimateIntegration.
  (return ""))