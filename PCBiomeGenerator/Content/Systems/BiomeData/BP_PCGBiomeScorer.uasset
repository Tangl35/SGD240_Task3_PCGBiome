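; PCG Blueprint element that scores climate data on each point to assign a biome type and weight.
; Reads climate and terrain attributes, then scores forest, grassland, freshwater, cliff, road fence and fog zone.
; Blended scores feed ChooseFinalBiome, whose weight is written to BiomeWeight.
; BiomeType is written without the chosen biome connected, FogDensity is read but unused, and fog scoring uses a fixed TimeOfDay.
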(fn ExecutewithContext
  (params (InContext :type PCG%20Context%20Structure%20%28by%20ref%29) (Input :type PCG%20Data%20Collection%20Structure%20%28by%20ref%29))
  (bind _returnvalue (Class|PCGBlueprintHelpers|GetInputData InContext))
  (bind _aspcgpoint_data (Utilities|Casting|CastToPCGPointData _returnvalue))
  (for _array_element (SpatialData|GetPoints _aspcgpoint_data) :!label _label ; Get Climate Attributes per point data
    ;[0.15 0.15 0.15 0.5] Get Climate Attributes
    (bind _returnvalue_2 (Ability|Attribute|GetFloatAttribute _array_element 0 "Temperature"))
    (bind _returnvalue_3 (Ability|Attribute|GetFloatAttribute _array_element 0 "Humidity"))
    (bind _returnvalue_4 (Ability|Attribute|GetFloatAttribute _array_element 0 "SlopeFactor"))
    (bind _returnvalue_5 (Ability|Attribute|GetFloatAttribute _array_element 0 "Elevation"))
    (bind _returnvalue_6 (Ability|Attribute|GetFloatAttribute _array_element 0 "WaterProximity"))
    (Ability|Attribute|GetFloatAttribute _array_element 0 "FogDensity")
    ;[0.15 0.15 0.15 0.5] Calculate BiomeScore
    (bind _score (CallFunction|ScoreRoadFence _returnvalue_2 _returnvalue_3 _returnvalue_4))
    (bind _score_2 (CallFunction|ScoreCliff _returnvalue_4 _returnvalue_5))
    (bind _score_3 (CallFunction|ScoreFreshwater _returnvalue_2 _returnvalue_3 _returnvalue_4 _returnvalue_6))
    (bind _score_4 (CallFunction|ScoreForest _returnvalue_2 _returnvalue_3 _returnvalue_4 _returnvalue_6))
    (bind _score_5 (CallFunction|ScoreGrassland _returnvalue_2 _returnvalue_3 _returnvalue_4 _returnvalue_6))
    (bind _score_6 (CallFunction|ScoreFogZone _returnvalue_3 _returnvalue_5 0.0))
    ;[0.15 0.15 0.15 0.5] BlendBiomeScores and ChooseFinalBiome for point
    (bind (_wforest _wgrassland _wfreshwater _wcliff _weightroadfence _wfogzone) (CallFunction|BlendBiomeScores _score_4 _score_5 _score_3 _score_2 _score _score_6))
    (bind _chosenweight (CallFunction|ChooseFinalBiome _wforest _wgrassland _wfreshwater _wcliff _weightroadfence _wfogzone))
    (Class|PCGMetadataAccessorHelpers|SetInteger64Attribute _array_element 0 "BiomeType") ; Enum to Int node needed ...?
    (PCG|Metadata|SetFloatAttribute _array_element 0 "BiomeWeight" _chosenweight)
    (goto _label))
  (SpatialData|SetPoints _aspcgpoint_data (SpatialData|GetPoints _aspcgpoint_data))
  (return ""))