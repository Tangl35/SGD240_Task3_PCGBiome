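; BP_WaterActor represents a body of water (lake, river, stream or pond) with functions for closest-point and proximity queries.
; GetClosestPointToWorldPosition returns the nearest RiverSpline point for both lakes and rivers.
; GetProximity subtracts lake radius or river half-width from horizontal distance, with stream and pond using zero-distance placeholders.
; Its clamped InfluenceRadius falloff return is disconnected, and the event graph is empty.
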(fn `GetClosestPointToWorldPosition`
  (params (WorldPosition :type "Vector Structure"))
  (returns (ClosestPoint :type "Vector Structure"))
  (bind _riverspline (`self.RiverSpline`))
  (switch `/Game/Systems/EWaterType` (`self.WaterType`)
    (:`NewEnumerator0`
      _)
    (:`NewEnumerator1`
      _))
  (return (`KismetMathLibrary.SelectVector` (`self.K2_GetActorLocation`) (`SplineComponent.GetLocationAtSplineInputKey` _riverspline (`SplineComponent.FindInputKeyClosestToWorldLocation` _riverspline WorldPosition) "World"))))

(fn `GetProximity`
  (params (WorldPosition :type "Vector Structure"))
  (returns (Proximity :type "Float (double-precision)"))
  (locals (EffectiveDistance :type "Float (double-precision)" :default 0.0))
  (bind _closestpoint (`self.GetClosestPointToWorldPosition` WorldPosition))
  (switch `/Game/Systems/EWaterType` (`self.WaterType`)
    (:`NewEnumerator0`
      (bind (_returnvalue_x _returnvalue_y) (`KismetMathLibrary.BreakVector` (- _closestpoint WorldPosition)))
      (bind _returnvalue (`KismetMathLibrary.VSize` (`KismetMathLibrary.MakeVector` _returnvalue_x _returnvalue_y)))
      (bind _output_get (set `local.EffectiveDistance` (`KismetMathLibrary.FMax` (- _returnvalue (`self.Lake Radius`))))))
    (:`NewEnumerator1`
      (bind _output_get_2 (set `local.EffectiveDistance` (`KismetMathLibrary.FMax` (- _returnvalue (`self.RiverHalfWidth`))))))
    (:`NewEnumerator2`
      ; Using Lake radius and River Half Width for now.
      (set `local.EffectiveDistance` (`KismetMathLibrary.FMax` (- 0.0 (`self.RiverHalfWidth`)))))
    (:`NewEnumerator3`
      (set `local.EffectiveDistance` (`KismetMathLibrary.FMax` (- 0.0 (`self.Lake Radius`)))))))

(fn `UserConstructionScript`)