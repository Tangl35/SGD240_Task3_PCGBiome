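; Biome scoring function library that rates forest, grassland, freshwater, cliff, road/fence and fog zone from environmental inputs like temperature, humidity, slope and elevation.
; Each score function clamps a weighted sum of its inputs to 0–1.
; BlendBiomeScores normalizes the six scores into weights when their total exceeds a small epsilon, with no fallback yet.
; ChooseFinalBiome is unfinished, returning a fixed biome at zero weight while its override-threshold and max-weight logic stays disconnected.
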(fn `BlendBiomeScores`
  (params (ScoreForest :type "Float (double-precision)") (ScoreGrassland :type "Float (double-precision)") (ScoreFreshwater :type "Float (double-precision)") (ScoreCliff :type "Float (double-precision)") (ScoreRoadFence :type "Float (double-precision)") (ScoreFogZone :type "Float (double-precision)"))
  (returns (WForest :type "Float (double-precision)") (WGrassland :type "Float (double-precision)") (WFreshwater :type "Float (double-precision)") (WCliff :type "Float (double-precision)") (WeightRoadFence :type "Float (double-precision)") (WFogZone :type "Float (double-precision)"))
  (bind _returnvalue (+ (+ (+ (+ (+ ScoreRoadFence ScoreCliff) ScoreFreshwater) ScoreForest) ScoreGrassland) ScoreFogZone))
  (if (> _returnvalue 0.001)
    (return (/ ScoreForest _returnvalue) (/ ScoreGrassland _returnvalue) (/ ScoreFreshwater _returnvalue) (/ ScoreCliff _returnvalue) (/ ScoreRoadFence _returnvalue) (/ ScoreFogZone _returnvalue))))

(fn `ChooseFinalBiome`
  (params (WForest :type "Float (double-precision)") (WGrassland :type "Float (double-precision)") (WFreshwater :type "Float (double-precision)") (WCliff :type "Float (double-precision)") (WRoadFence :type "Float (double-precision)") (WFogDensity :type "Float (double-precision)"))
  (returns (ChosenBiome :type "/Game/Systems/EBiomeTypes Enum") (ChosenWeight :type "Float (double-precision)"))
  (locals (CliffOverrideThreshold :type "Float (double-precision)" :default 0.7) (WaterOverrideThreshold :type "Float (double-precision)" :default 0.7) (RoadOverrideThreshold :type "Float (double-precision)" :default 0.6) (MaxScore :type "Float (double-precision)") (MaxIndex :type Integer))
  (return "NewEnumerator4" 0.0))

(fn `ScoreCliff`
  (params (Slope :type "Float (double-precision)") (Elevation :type "Float (double-precision)"))
  (returns (Score :type "Float (double-precision)"))
  (return (`KismetMathLibrary.FClamp` (+ (* (- Slope 0.6) 2.0) (* Elevation 0.1)))))

(fn `ScoreFogZone`
  (params (Humidity :type "Float (double-precision)") (Elevation :type "Float (double-precision)") (TimeOfDay :type "Float (double-precision)"))
  (returns (Score :type "Float (double-precision)"))
  (return (`KismetMathLibrary.FClamp` (+ (+ (* Humidity 0.8) (* (- 1.0 Elevation) 0.1)) (* TimeOfDay 0.1)))))

(fn `ScoreForest`
  (params (Temperature :type "Float (double-precision)") (Humidity :type "Float (double-precision)") (Slope :type "Float (double-precision)") (WaterProximity :type "Float (double-precision)"))
  (returns (Score :type "Float (double-precision)"))
  (return (`KismetMathLibrary.FClamp` (+ (+ (+ (* (`KismetMathLibrary.FMax` (- Temperature 0.35)) 1.5) (* (`KismetMathLibrary.FMax` (- Humidity 0.55)) 2.0)) (* (`KismetMathLibrary.FClamp` (- 1.0 Slope)) 0.6)) (* WaterProximity 0.3)))))

(fn `ScoreFreshwater`
  (params (Temperature :type "Float (double-precision)") (Humidity :type "Float (double-precision)") (Slope :type "Float (double-precision)") (WaterProximity :type "Float (double-precision)"))
  (returns (Score :type "Float (double-precision)"))
  (return (`KismetMathLibrary.FClamp` (+ (* (- Slope 0.0) 0.3) (* WaterProximity 2.0)))))

(fn `ScoreGrassland`
  (params (Temperature :type "Float (double-precision)") (Humidity :type "Float (double-precision)") (Slope :type "Float (double-precision)") (WaterProximity :type "Float (double-precision)"))
  (returns (Score :type "Float (double-precision)"))
  (return (`KismetMathLibrary.FClamp` (+ (+ (+ (* (`KismetMathLibrary.FMax` (- Temperature 0.25)) 1.0) (* (`KismetMathLibrary.FMax` (- 0.6 Humidity)) 0.8)) (* (- 1.0 Slope) 4.0)) (* WaterProximity 0.5)))))

(fn `ScoreRoadFence`
  (params (Temperature :type "Float (double-precision)") (Humidity :type "Float (double-precision)") (Slope :type "Float (double-precision)"))
  (returns (Score :type "Float (double-precision)"))
  (return (`KismetMathLibrary.FClamp` (* Slope 0.4))))